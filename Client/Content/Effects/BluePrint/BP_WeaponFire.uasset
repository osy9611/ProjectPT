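; Weapon fire effects actor that plays Niagara shell eject, muzzle flash and tracer effects when Fire is called.
; Each system spawns attached at a socket offset, is reused while active, and replays by flipping its User.Trigger bool.
; Impact positions aim the flash and feed the tracer array.
; A retriggerable delay loop destroys the actor once shell eject and tracer components are invalid; muzzle flash is not checked.
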(event `Fire`
  (params (MuzzleTransform :type "SkeletalMeshComponent Object Reference"))
  (bind _ns_shelleject (`self.NS_ShellEject`))
  (bind _ns_muzzleflash (`self.NS_MuzzleFlash`))
  (bind _ns_tracer (`self.NS_Tracer`))
  (set `self.Muzzle Transform` MuzzleTransform)
  (`|ExecutionSequence`
    (:`then_0`
      (if (`self.Enable Shell Eject`)
        (`/Engine/EditorBlueprintResources/StandardMacros.IsValid` _ns_shelleject
          (:`Is Valid`
            (if (not (`ActorComponent.IsActive` _ns_shelleject))
              (bind _returnvalue (`NiagaraFunctionLibrary.SpawnSystemAttached` (`self.Shell Eject System`) (`self.DefaultSceneRoot`) "None" (.location (`SceneComponent.GetSocketTransform` (`self.Skeletal Mesh Component`) "Shell Effect" "RTS_Actor")) (`KismetMathLibrary.MakeRotator` 0.0 0.0 0.0) "KeepRelativeOffset" true :!label _label))
              (bind _output_get (set `self.NS_ShellEject` _returnvalue))
              (`NiagaraComponent.SetVariableStaticMesh` _output_get "User.ShellEjectStaticMesh" (`self.Shell Eject Mesh`))
              (set `self.Shell Eject Trigger` false)))
          (:`Is Not Valid`
            (goto _label)))
        (set `self.Shell Eject Trigger` (not (`self.Shell Eject Trigger`)))
        (`NiagaraComponent.SetVariableBool` (`self.NS_ShellEject`) "User.Trigger" (`self.Shell Eject Trigger`))))
    (:`then_1`
      (if (`self.Enable Muzzle Flash`)
        (`/Engine/EditorBlueprintResources/StandardMacros.IsValid` _ns_muzzleflash
          (:`Is Valid`
            (if (not (`ActorComponent.IsActive` _ns_muzzleflash))
              (bind _returnvalue_2 (`NiagaraFunctionLibrary.SpawnSystemAttached` (`self.Muzzle Flash System`) (`self.DefaultSceneRoot`) "None" (.location (`SceneComponent.GetSocketTransform` (`self.Muzzle Transform`) (`self.Muzzle Name`) "RTS_Actor")) (`KismetMathLibrary.MakeRotator` 0.0 0.0 0.0) "KeepRelativeOffset" true :!label _label_2))
              (set `self.NS_MuzzleFlash` _returnvalue_2)
              (set `self.Shell Eject Trigger` false)))
          (:`Is Not Valid`
            (goto _label_2)))
        (set `self.Muzzle Flash Trigger` (not (`self.Muzzle Flash Trigger`)))
        (`NiagaraComponent.SetVariableBool` (`self.NS_MuzzleFlash`) "User.Trigger" (`self.Muzzle Flash Trigger`))
        (`NiagaraComponent.SetVariableVec3` (`self.NS_MuzzleFlash`) "User.Direction" (`KismetMathLibrary.Normal` (- (`|GetArrayItem` (`self.Impact Positions`)) (.location (`SceneComponent.GetSocketTransform` (`self.Muzzle Transform`) (`self.Muzzle Name`) "RTS_World")))))))
    (:`then_2`
      (if true
        (`/Engine/EditorBlueprintResources/StandardMacros.IsValid` _ns_tracer
          (:`Is Valid`
            (if (not (`ActorComponent.IsActive` _ns_tracer))
              (bind _returnvalue_3 (`NiagaraFunctionLibrary.SpawnSystemAttached` (`self.Tracer System`) (`self.DefaultSceneRoot`) "None" (.location (`SceneComponent.GetSocketTransform` (`self.Muzzle Transform`) (`self.Muzzle Name`) "RTS_Actor")) (`KismetMathLibrary.MakeRotator` 0.0 0.0 0.0) "KeepRelativeOffset" :!label _label_3))
              (set `self.NS_Tracer` _returnvalue_3)
              (set `self.Tracer Trigger` false)))
          (:`Is Not Valid`
            (goto _label_3)))
        (set `self.Tracer Trigger` (not (`self.Tracer Trigger`)))
        (`NiagaraComponent.SetVariableBool` (`self.NS_Tracer`) "User.Trigger" (`self.Tracer Trigger`))
        (`NiagaraDataInterfaceArrayFunctionLibrary.SetNiagaraArrayVector` (`self.NS_Tracer`) "User.ImpactPositions" (`self.Impact Positions`))))
    (:`then_3`
      (`KismetSystemLibrary.RetriggerableDelay` 3.0 :!label _label_4)
      (if (or (`KismetSystemLibrary.IsValid` (`self.NS_ShellEject`)) (`KismetSystemLibrary.IsValid` (`self.NS_ShellEject`)) (`KismetSystemLibrary.IsValid` (`self.NS_Tracer`)))
        (goto _label_4)
        (else
          (`self.K2_DestroyActor`))))))

(fn `UserConstructionScript`)