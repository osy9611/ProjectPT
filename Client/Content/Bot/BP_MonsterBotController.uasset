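; AI controller for monster bots that runs a behavior tree on possess and feeds it enemy targets from AI perception.
; A sensed Player-tagged actor sets EnemyActor and HasLineOfSight in the Blackboard if visible, or regardless once the bot is attacked.
; Stimuli tagged AI.Event.Attack set both keys immediately and latch IsAttacked, which nothing here resets.
; Neither handler clears the keys.
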(event `self.ReceivePossess`
  (params (PossessedPawn :type "Pawn Object Reference"))
  (`self.RunBehaviorTree` (`self.BTAsset`)))

(event `self.AIPerceptionComponent.OnTargetPerceptionUpdated`
  (params (Actor :type "Actor Object Reference") (Stimulus :type "AIStimulus Structure"))
  (set `self.TargetActor` Actor)
  (if (and (`self.ActorHasTag` Actor "Player") (`.bSuccessfullySensed` (break `AIStimulus` Stimulus)))
    (bind _returnvalue (`PTAIComponent.IsTargetVisible` (`self.AIComponent`) (`self.TargetActor`)))
    (if _returnvalue
      (`BlackboardComponent.SetValueAsBool` (`self.Blackboard`) (`self.Has Line Of Sight`) true :!label _label)
      (`BlackboardComponent.SetValueAsObject` (`self.Blackboard`) (`self.Enemy Actor`) (`self.TargetActor`))
      (elif (`self.IsAttacked`)
        (goto _label)))))

(event `self.AIPerceptionComponent.OnTargetPerceptionInfoUpdated`
  (params (UpdateInfo :type "ActorPerceptionUpdateInfo Structure (by ref)"))
  (bind (_result _actor) (`self.CheckGameplayTag` UpdateInfo (struct :`TagName` "AI.Event.Attack")))
  (if _result
    (`BlackboardComponent.SetValueAsBool` (`self.Blackboard`) (`self.Has Line Of Sight`) true)
    (`BlackboardComponent.SetValueAsObject` (`self.Blackboard`) (`self.Enemy Actor`) _actor)
    (set `self.IsAttacked` true)))

(fn `CheckGameplayTag`
  (params (UpdateInfo :type "ActorPerceptionUpdateInfo Structure") (GameplayTag :type "GameplayTag Structure"))
  (returns (Result :type Boolean) (Actor :type "Actor Object Reference"))
  (bind ((`Target` _target) (`Stimulus` _stimulus)) (break `ActorPerceptionUpdateInfo` UpdateInfo))
  (return (== (`BlueprintGameplayTagLibrary.GetTagName` GameplayTag) (`.Tag` (break `AIStimulus` _stimulus))) _target))

(fn `CheckGameplayTagByName`
  (params (TagName :type Name) (CheckTag :type "GameplayTag Structure"))
  (returns (Result :type Boolean))
  (return (== TagName (`BlueprintGameplayTagLibrary.GetTagName` CheckTag))))

(fn `UserConstructionScript`)