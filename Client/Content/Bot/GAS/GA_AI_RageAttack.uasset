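; Gameplay ability for an AI bot's rage attack, a montage-driven ranged attack.
; On activation it reads damage from tagged skill data, plays the montage, then starts ranged targeting after a delay.
; When target data arrives, it sets the monster skill's muzzle, applies damage and fires a gameplay cue from the first hit.
; The ability ends when the fire timer elapses or the montage completes, is interrupted or cancelled.
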(event `self.K2_ActivateAbility`
  (`|ExecutionSequence`
    (:`then_0`
      (bind _returnvalue (`self.GetGameplayTag`))
      (bind _returnvalue_2 (`self.GetPTAttribute`))
      (bind _returnvalue_3 (`PTAttributeSet.GetSkillData` _returnvalue_2 _returnvalue))
      (set `self.Damage` (`.SkillDamage` (break `SkillData` _returnvalue_3))))
    (:`then_1`
      (`AbilityTask_PlayMontageAndWait.CreatePlayMontageAndWaitProxy` "None" (`self.AnimMontage`)
        (:`then`
          (`AbilityTask_WaitDelay.WaitDelay` (`self.Check Fire Time`)
            (:`OnFinish`
              (`self.StartRangedWeaponTargeting`)
              (`KismetSystemLibrary.K2_SetTimerDelegate` (delegate `FireComplete`) (`self.Fire Delay Time`)))))
        (:`OnCompleted`
          (`self.K2_EndAbility` :!label _label))
        (:`OnInterrupted`
          (goto _label))
        (:`OnCancelled`
          (goto _label))))))

(event `FireComplete`
  (goto _label))

(event `self.OnRangeWeaponTargetDataReady`
  (params (Owner :type "Actor Object Reference") (TargetData :type "GameplayAbilityTargetDataHandle Structure (by ref)"))
  (bind _asbp_monster_bot (cast `/Game/Bot/BP_MonsterBot` Owner))
  (bind _asbp_skill (cast `/Game/Characters/BP_Skill` (`/Game/Bot/BP_MonsterBot.Skill` _asbp_monster_bot)))
  (bind _returnvalue (`self.GetMuzzleName`))
  (set `/Game/Characters/BP_Skill.Muzzle Name` _returnvalue _asbp_skill)
  (set `/Game/Characters/BP_Skill.Target Skeletal Mesh` null _asbp_skill)
  (set `self.GCNParameter` (`GameplayCueFunctionLibrary.MakeGameplayCueParametersFromHitResult` (`AbilitySystemBlueprintLibrary.GetHitResultFromTargetData` TargetData)))
  (`PTObjectSubsystem.ApplyActorsDamage` (subsystem `PTObjectSubsystem`) (`self.GetOwningActorFromActorInfo`) TargetData (`self.Damage`))
  (`self.K2_ExecuteGameplayCueWithParams` (`self.Gameplay Cue Tag Firing`) (`self.GCNParameter`)))