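; BP_Skill is a skill Blueprint that drives weapon firing effects through a helper BP_WeaponFire actor.
; Fire stores impact data, then gets the RootActor's skeletal mesh and its muzzle socket transform via PTPawnExtensionComponent.
; It lazily spawns and attaches one BP_WeaponFire configured with muzzle flash, shell eject and tracer assets, then passes it the impacts and target mesh on each shot.
; A WeaponImpact validity check is left unconnected.
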(event `Fire`
  (params (`Impact Position` :type "Array of Vector Structure") (`Impact Normals` :type "Array of Vector Structure") (`Impact Surface Types` :type "Array of EPhysicalSurface Enum") (RootActor :type "Actor Object Reference"))
  (set `self.Impact Position` `Impact Position`)
  (set `self.Impact Normals` `Impact Normals`)
  (set `self.Impact Surface Types` `Impact Surface Types`)
  (set `self.Target Skeletal Mesh` (`self.GetComponentByClass` RootActor "/Script/Engine.SkeletalMeshComponent"))
  (bind _returnvalue (`PTPawnExtensionComponent.GetSkeletonMeshSocketTransform` (`self.GetComponentByClass` RootActor "/Script/ProjectPT.PTPawnExtensionComponent") (`KismetStringLibrary.Conv_StringToName` (`self.Muzzle Name`))))
  (set `self.Muzzle Position` _returnvalue)
  (`|ExecutionSequence`
    (:`then_0`
      ;[1 1 1] Weapon Fire
      (`/Engine/EditorBlueprintResources/StandardMacros.IsValid` (`self.Weapon Fire`)
        (:`Is Valid`
          _)
        (:`Is Not Valid`
          (bind _returnvalue_2 (`|SpawnActorFromClass` "/Game/Effects/BluePrint/BP_WeaponFire.BP_WeaponFire_C" (`KismetMathLibrary.MakeTransform` (0.0 0.0 0.0)) "Undefined" "MultiplyWithRoot" null true (`self.Muzzle Flash System`) true (`KismetStringLibrary.Conv_StringToName` (`self.Muzzle Name`)) true (`self.SkeletalMesh`) (`self.Shell Eject System`) (`self.Shell Eject Mesh`) (`self.Tracer System`) null))
          (bind _output_get (set `self.Weapon Fire` _returnvalue_2))
          (`self.K2_AttachToComponent` _output_get (`self.SkeletalMesh`) "None" "KeepRelative" "KeepRelative" "KeepRelative" true)))
      (set `/Game/Effects/BluePrint/BP_WeaponFire.Impact Positions` (`self.Impact Position`) (`self.Weapon Fire`))
      (set `/Game/Effects/BluePrint/BP_WeaponFire.Impact Normals` (`self.Impact Normals`) (`self.Weapon Fire`))
      (set `/Game/Effects/BluePrint/BP_WeaponFire.Impact Surface Types` (`self.Impact Surface Types`) (`self.Weapon Fire`))
      (`/Game/Effects/BluePrint/BP_WeaponFire.Fire` (`self.Weapon Fire`) (`self.Target Skeletal Mesh`)))))

(fn `UserConstructionScript`)